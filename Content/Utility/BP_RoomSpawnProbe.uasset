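; Procedural floor-generation probe that loads a random room level instance at its grid location.
; On BeginPlay it registers that cell in the GameInstance, caches room pools and computes forward, right and left neighbor cells.
; Intermediate spawns check those neighbors to pick a fitting room type and 90-degree rotation.
; Boss, treasure, shop and endcap events load special rooms, with most reporting to BP_FloorMaster to chain or retry stages; successful probes destroy themselves.
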(event EventBeginPlay
  (bind _asmy_game_instance (Utilities|Casting|CastToMyGameInstance (Game|GetGameInstance))
    (:then
      (Variables|Default|SetGameInstanceRef _asmy_game_instance)
      (Utilities|FlowControl|Delay 0.2)
      (Variables|Default|SetRoomSize (Variables|/Game/Utility/MyGameInstance.MyGameInstance_C|GetRoomSize (Variables|Default|GetGameInstanceRef)))
      (bind _intvector (CallFunction|FloatVectortoIntVector (Transformation|GetWorldLocation (Variables|Default|GetSphere)) (Math|Conversions|ToFloat(Integer) (Variables|Default|GetRoomSize))))
      (Variables|Default|SetLocation _intvector)
      (if (== (Utilities|Array|FindItem (Variables|/Game/Utility/MyGameInstance.MyGameInstance_C|GetRoomLocationsTakenInt (Variables|Default|GetGameInstanceRef)) (Variables|Default|GetLocation)) -1)
        (Utilities|Array|Add (Variables|/Game/Utility/MyGameInstance.MyGameInstance_C|GetRoomLocationsTakenInt (Variables|Default|GetGameInstanceRef)) (Variables|Default|GetLocation))
        (if (== (Utilities|Array|FindItem (Variables|/Game/Utility/MyGameInstance.MyGameInstance_C|GetRoomLocationsMinimap (Variables|Default|GetGameInstanceRef)) (Variables|Default|GetLocation)) -1)
          (Utilities|Array|Add (Variables|/Game/Utility/MyGameInstance.MyGameInstance_C|GetRoomLocationsMinimap (Variables|Default|GetGameInstanceRef)) (Variables|Default|GetLocation))
          (Utilities|LoadLevels)
          (bind _intvector_2 (CallFunction|FloatVectortoIntVector (Math|Vector|GetForwardVector (Variables|Default|GetForwardArrow)) 1.0))
          (bind _outvector (CallFunction|MultiplybyInt _intvector_2 (Variables|Default|GetRoomSize)))
          (bind _outvector_2 (CallFunction|IntVector+IntVector _outvector (Utilities|RoundIntVector (Variables|Default|GetLocation))))
          (Variables|CardinalDirectionsVectors|SetForwardLocation _outvector_2)
          (bind _intvector_3 (CallFunction|FloatVectortoIntVector (Math|Vector|GetForwardVector (Variables|Default|GetRightArrow)) 1.0))
          (bind _outvector_3 (CallFunction|MultiplybyInt _intvector_3 (Variables|Default|GetRoomSize)))
          (bind _outvector_4 (CallFunction|IntVector+IntVector _outvector_3 (Variables|Default|GetLocation)))
          (Variables|CardinalDirectionsVectors|SetRightLocation _outvector_4)
          (bind _intvector_4 (CallFunction|FloatVectortoIntVector (Math|Vector|GetForwardVector (Variables|Default|GetLeftArrow)) 1.0))
          (bind _outvector_5 (CallFunction|MultiplybyInt _intvector_4 (Variables|Default|GetRoomSize)))
          (bind _outvector_6 (CallFunction|IntVector+IntVector _outvector_5 (Variables|Default|GetLocation)))
          (Variables|CardinalDirectionsVectors|SetLeftLocation _outvector_6))))
    (:CastFailed
      (Development|PrintString "Cast to MyGameInstance failed" true true "(R=1.000000,G=0.000000,B=0.007957,A=1.000000)" 15.0))))

(event EventSpawnIntermediateRoom
  (Utilities|FlowControl|Sequence
    (:then_0
      (if (!= (Utilities|Array|FindItem (Variables|/Game/Utility/MyGameInstance.MyGameInstance_C|GetRoomLocationsTakenInt (Variables|Default|GetGameInstanceRef)) (Variables|CardinalDirectionsVectors|GetForwardLocation)) -1)
        (Variables|CardinalDirections|SetIsForwardFree false)
        (else
          (Variables|CardinalDirections|SetIsForwardFree true))))
    (:then_1
      (if (!= (Utilities|Array|FindItem (Variables|/Game/Utility/MyGameInstance.MyGameInstance_C|GetRoomLocationsTakenInt (Variables|Default|GetGameInstanceRef)) (Variables|CardinalDirectionsVectors|GetRightLocation)) -1)
        (Variables|CardinalDirections|SetIsRightFree false)
        (else
          (Variables|CardinalDirections|SetIsRightFree true))))
    (:then_2
      (if (!= (Utilities|Array|FindItem (Variables|/Game/Utility/MyGameInstance.MyGameInstance_C|GetRoomLocationsTakenInt (Variables|Default|GetGameInstanceRef)) (Variables|CardinalDirectionsVectors|GetLeftLocation)) -1)
        (Variables|CardinalDirections|SetIsLeftFree false)
        (else
          (Variables|CardinalDirections|SetIsLeftFree true))))
    (:then_3
      ;[1 1 1] Is FORWARD free?
      (if (Variables|CardinalDirections|GetIsForwardFree)
        ;[1 1 1] Is RIGHT free?
        (if (Variables|CardinalDirections|GetIsRightFree)
          ;[1 1 1] Is LEFT free?
          (if (Variables|CardinalDirections|GetIsLeftFree)
            (switch int (Math|Random|RandomIntegerinRange 0 3)
              (:0
                (bind (_boutsuccess _returnvalue) (Utilities|SpawnRoom (Variables|RoomArrays|GetCrossroads) (Math|Random|RandomIntegerinRange 0 3)))
                (Utilities|Array|Add (Variables|/Game/Utility/MyGameInstance.MyGameInstance_C|GetLoadedRoomsList (Variables|Default|GetGameInstanceRef)) _returnvalue)
                (if _boutsuccess
                  (bind _outactors (Actor|GetAllActorsOfClass "/Game/Utility/BP_FloorMaster.BP_FloorMaster_C" :!label _label))
                  (bind _result (Math|Integer|IncrementInt (Variables|/Game/Utility/BP_FloorMaster.BP_FloorMaster_C|GetProbeIndex (Utilities|Array|Get(acopy) _outactors)))
                    (:%20%20
                      (Variables|/Game/Utility/BP_FloorMaster.BP_FloorMaster_C|SetProbeIndex (Utilities|Array|Get(acopy) _outactors) _result)
                      (Actor|DestroyActor)))
                  (else
                    (Actor|DestroyActor :!label _label_2))))
              (:1
                (Variables|Default|SetMinRot -1)
                (Variables|Default|SetMaxRot 1)
                (bind (_boutsuccess_2 _returnvalue_2) (Utilities|SpawnRoom (Variables|RoomArrays|GetT-splits) (Math|Random|RandomIntegerinRange (Variables|Default|GetMinRot) (Variables|Default|GetMaxRot)) :!label _label_3))
                (Utilities|Array|Add (Variables|/Game/Utility/MyGameInstance.MyGameInstance_C|GetLoadedRoomsList (Variables|Default|GetGameInstanceRef)) _returnvalue_2)
                (if _boutsuccess_2
                  (goto _label)
                  (else
                    (goto _label_2))))
              (:2
                (Variables|Default|SetMinRot 0)
                (Variables|Default|SetMaxRot 1)
                (bind (_boutsuccess_3 _returnvalue_3) (Utilities|SpawnRoom (Variables|RoomArrays|GetL-bends) (Math|Random|RandomIntegerinRange (Variables|Default|GetMinRot) (Variables|Default|GetMaxRot)) :!label _label_4))
                (Utilities|Array|Add (Variables|/Game/Utility/MyGameInstance.MyGameInstance_C|GetLoadedRoomsList (Variables|Default|GetGameInstanceRef)) _returnvalue_3)
                (if _boutsuccess_3
                  (goto _label)
                  (else
                    (goto _label_2))))
              (:3
                (bind (_boutsuccess_4 _returnvalue_4) (Utilities|SpawnRoom (Variables|RoomArrays|GetCorridors) (* (Math|Random|RandomIntegerinRange 0 1) 2) :!label _label_5))
                (Utilities|Array|Add (Variables|/Game/Utility/MyGameInstance.MyGameInstance_C|GetLoadedRoomsList (Variables|Default|GetGameInstanceRef)) _returnvalue_4)
                (if _boutsuccess_4
                  (goto _label)
                  (else
                    (goto _label_2)))))
            (else
              (switch int (Math|Random|RandomIntegerinRange 0 2)
                (:0
                  (Variables|Default|SetMinRot -1)
                  (Variables|Default|SetMaxRot -1)
                  (goto _label_3))
                (:1
                  (Variables|Default|SetMinRot 0)
                  (Variables|Default|SetMaxRot 0)
                  (goto _label_4))
                (:2
                  (goto _label_5)))))
          (elif (Variables|CardinalDirections|GetIsLeftFree)
            (switch int (Math|Random|RandomIntegerinRange 0 2)
              (:0
                (Variables|Default|SetMinRot 1)
                (Variables|Default|SetMaxRot 1)
                (goto _label_3))
              (:1
                (Variables|Default|SetMinRot 1)
                (Variables|Default|SetMaxRot 1)
                (goto _label_4))
              (:2
                (goto _label_5)))
            (else
              (goto _label_5))))
        (elif (Variables|CardinalDirections|GetIsRightFree)
          (if (Variables|CardinalDirections|GetIsLeftFree)
            (switch int (Math|Random|RandomIntegerinRange 0 2)
              (:0
                (Variables|Default|SetMinRot 0)
                (Variables|Default|SetMaxRot 0)
                (goto _label_3))
              (:1
                (Variables|Default|SetMinRot 0)
                (Variables|Default|SetMaxRot 1)
                (goto _label_4)))
            (else
              (Variables|Default|SetMinRot 0)
              (Variables|Default|SetMaxRot 0)
              (goto _label_4)))
          (elif (Variables|CardinalDirections|GetIsLeftFree)
            (Variables|Default|SetMinRot 1)
            (Variables|Default|SetMaxRot 1)
            (goto _label_4)
            (else
              (bind (_boutsuccess_5 _returnvalue_5) (Utilities|SpawnRoom (Variables|RoomArrays|GetEndcaps)))
              (Utilities|Array|Add (Variables|/Game/Utility/MyGameInstance.MyGameInstance_C|GetLoadedRoomsList (Variables|Default|GetGameInstanceRef)) _returnvalue_5)
              (if _boutsuccess_5
                (goto _label)
                (else
                  (goto _label_2))))))))))

(event EventSpawnEndRoom
  (bind (_boutsuccess _returnvalue) (Utilities|SpawnRoom (Variables|RoomArrays|GetEndcaps)))
  (Utilities|Array|Add (Variables|/Game/Utility/MyGameInstance.MyGameInstance_C|GetLoadedRoomsList (Variables|Default|GetGameInstanceRef)) _returnvalue)
  (if _boutsuccess
    (Actor|DestroyActor)))

(event EventSpawnBossRoom
  (bind (_boutsuccess _returnvalue) (Utilities|SpawnRoom (Variables|RoomArrays|GetBossArenas)))
  (Utilities|Array|Add (Variables|/Game/Utility/MyGameInstance.MyGameInstance_C|GetLoadedRoomsList (Variables|Default|GetGameInstanceRef)) _returnvalue)
  (if _boutsuccess
    (bind _outactors (Actor|GetAllActorsOfClass "/Game/Utility/BP_FloorMaster.BP_FloorMaster_C"))
    (Class|ISpawnsRooms|ReSpawnTreasureRoom(Message) (Utilities|Array|Get(acopy) _outactors))
    (Actor|DestroyActor)
    (else
      (bind _outactors_2 (Actor|GetAllActorsOfClass "/Game/Utility/BP_FloorMaster.BP_FloorMaster_C"))
      (Class|ISpawnsRooms|ReSpawnBossRoom(Message) (Utilities|Array|Get(acopy) _outactors_2))
      (Development|PrintString "Hello"))))

(event EventSpawnTreasureRoom
  (bind (_boutsuccess _returnvalue) (Utilities|SpawnRoom (Variables|RoomArrays|GetTreasureRooms)))
  (Utilities|Array|Add (Variables|/Game/Utility/MyGameInstance.MyGameInstance_C|GetLoadedRoomsList (Variables|Default|GetGameInstanceRef)) _returnvalue)
  (if _boutsuccess
    (bind _outactors (Actor|GetAllActorsOfClass "/Game/Utility/BP_FloorMaster.BP_FloorMaster_C"))
    (Class|ISpawnsRooms|ReSpawnShop(Message) (Utilities|Array|Get(acopy) _outactors))
    (Actor|DestroyActor)
    (else
      (bind _outactors_2 (Actor|GetAllActorsOfClass "/Game/Utility/BP_FloorMaster.BP_FloorMaster_C"))
      (Class|ISpawnsRooms|ReSpawnTreasureRoom(Message) (Utilities|Array|Get(acopy) _outactors_2)))))

(event EventSpawnShop
  (bind (_boutsuccess _returnvalue) (Utilities|SpawnRoom (Variables|RoomArrays|GetShops)))
  (Utilities|Array|Add (Variables|/Game/Utility/MyGameInstance.MyGameInstance_C|GetLoadedRoomsList (Variables|Default|GetGameInstanceRef)) _returnvalue)
  (if _boutsuccess
    (bind _outactors (Actor|GetAllActorsOfClass "/Game/Utility/BP_FloorMaster.BP_FloorMaster_C"))
    (Class|ISpawnsRooms|ReSpawnEndcaps(Message) (Utilities|Array|Get(acopy) _outactors))
    (Actor|DestroyActor)
    (else
      (bind _outactors_2 (Actor|GetAllActorsOfClass "/Game/Utility/BP_FloorMaster.BP_FloorMaster_C"))
      (Class|ISpawnsRooms|ReSpawnShop(Message) (Utilities|Array|Get(acopy) _outactors_2)))))

(fn ConstructionScript)