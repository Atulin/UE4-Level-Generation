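; BP_FloorMaster procedurally generates a floor from randomly picked level-instance rooms, tracking grid cells in MyGameInstance.
; After placing the first room, it messages BP_RoomSpawnProbe actors on delayed loops to add regular rooms, then a boss room.
; Re-entrant events handle treasure, shop and dead-end rooms, then spawn doors, rebuild navigation and broadcast loading end.
; LoadingEnds retries dead ends, then destroys all probes and itself.
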(event EventBeginPlay
  (bind _asmy_game_instance (Utilities|Casting|CastToMyGameInstance (Game|GetGameInstance))
    (:then
      (bind _output_get (Variables|Default|SetGameInstanceRef _asmy_game_instance))
      (Variables|Default|SetRoomSize (Variables|/Game/Utility/MyGameInstance.MyGameInstance_C|GetRoomSize _output_get))
      ;[1 1 1] Gets current room coordinates, checks if they aren't taken (they shouldn't be, it's the first probe in the level), adds current coordinates to the array of taken coordinates
      (bind _intvector (CallFunction|FloatVectortoIntVector (Transformation|GetWorldLocation (Variables|Default|GetSphere)) (Math|Conversions|ToFloat(Integer) (Variables|Default|GetRoomSize))))
      (Variables|Default|SetLocation _intvector)
      (if (== (Utilities|Array|FindItem (Variables|/Game/Utility/MyGameInstance.MyGameInstance_C|GetRoomLocationsTakenInt (Variables|Default|GetGameInstanceRef)) (Variables|Default|GetLocation)) -1)
        (Utilities|Array|Add (Variables|/Game/Utility/MyGameInstance.MyGameInstance_C|GetRoomLocationsTakenInt (Variables|Default|GetGameInstanceRef)) (Variables|Default|GetLocation))
        (Utilities|LoadLevels)
        (if (Variables|Default|GetIsFirstRoom?)
          (bind _returnvalue (Utilities|SpawnRoom (Variables|RoomArrays|GetFirstRooms) (* (Math|Random|RandomIntegerinRange 0 3) 90)))
          (Variables|/Game/Utility/MyGameInstance.MyGameInstance_C|SetStartRoomRef (Variables|Default|GetGameInstanceRef) _returnvalue)
          (else
            (bind _returnvalue_2 (Utilities|SpawnRoom (Variables|RoomArrays|GetFirstRooms) (* (Math|Random|RandomIntegerinRange 0 3) 90)))
            (Variables|/Game/Utility/MyGameInstance.MyGameInstance_C|SetStartRoomRef (Variables|Default|GetGameInstanceRef) _returnvalue_2)))
        (Utilities|UpdateLoadingText "Mapping the floor")
        ;[1 1 1] Sends message to a first probe from an always updating array, which means each iteration will spawn room on a different probe
        (if (== (Variables|/Game/Utility/MyGameInstance.MyGameInstance_C|GetNumberOfRooms (Variables|Default|GetGameInstanceRef)) (Variables|Default|GetProbeIndex)) :!label _label
          (Utilities|UpdateLoadingText "Initializing boss defence protocols")
          ;[1 1 1] When spawning regular rooms is done, time to start spawning special rooms – shop, treasure room and boss arena
          ;;[1 0 0] ¯\_(ツ)_/¯
          (Utilities|FlowControl|Delay 0.1)
          (bind _outactors (Actor|GetAllActorsOfClass "/Game/Utility/BP_RoomSpawnProbe.BP_RoomSpawnProbe_C"))
          (Class|ISpawnsRooms|SpawnBossRoom(Message) (Utilities|Array|Get(acopy) _outactors (Math|Random|RandomIntegerinRange 0 (Utilities|Array|LastIndex _outactors))))
          (else
            (bind _outactors_2 (Actor|GetAllActorsOfClass "/Game/Utility/BP_RoomSpawnProbe.BP_RoomSpawnProbe_C"))
            ;;[1 0 0] ¯\_(ツ)_/¯
            (Utilities|FlowControl|Delay 0.2)
            (Class|ISpawnsRooms|SpawnIntermediateRoom(Message) (Utilities|Array|Get(acopy) _outactors_2))
            (goto _label)))
        (else
          (Development|PrintString "5b"))))
    (:CastFailed
      (Development|PrintString "Cast to MyGameInstance failed" true true "(R=1.000000,G=0.000000,B=0.007957,A=1.000000)" 15.0))))

(event EventReSpawnBossRoom
  ;[1 1 1] When spawning regular rooms is done, time to start spawning special rooms – shop, treasure room and boss arena
  ;;[1 0 0] ¯\_(ツ)_/¯
  (Utilities|FlowControl|Delay 0.1)
  (bind _outactors (Actor|GetAllActorsOfClass "/Game/Utility/BP_RoomSpawnProbe.BP_RoomSpawnProbe_C"))
  (Class|ISpawnsRooms|SpawnBossRoom(Message) (Utilities|Array|Get(acopy) _outactors (Math|Random|RandomIntegerinRange 0 (Utilities|Array|LastIndex _outactors)))))

(event EventReSpawnTreasureRoom
  ;[1 1 1] When spawning regular rooms is done, time to start spawning special rooms – shop, treasure room and boss arena
  (Utilities|UpdateLoadingText "Taking stock of treasury")
  ;;[1 0 0] ¯\_(ツ)_/¯
  (Utilities|FlowControl|Delay 0.1)
  (bind _outactors (Actor|GetAllActorsOfClass "/Game/Utility/BP_RoomSpawnProbe.BP_RoomSpawnProbe_C"))
  (Class|ISpawnsRooms|SpawnTreasureRoom(Message) (Utilities|Array|Get(acopy) _outactors (Math|Random|RandomIntegerinRange 0 (Utilities|Array|LastIndex _outactors)))))

(event EventReSpawnShop
  ;[1 1 1] When spawning regular rooms is done, time to start spawning special rooms – shop, treasure room and boss arena
  (Utilities|UpdateLoadingText "Attempting to initialize shop system")
  ;;[1 0 0] ¯\_(ツ)_/¯
  (Utilities|FlowControl|Delay 0.1)
  (bind _outactors (Actor|GetAllActorsOfClass "/Game/Utility/BP_RoomSpawnProbe.BP_RoomSpawnProbe_C"))
  (Class|ISpawnsRooms|SpawnShop(Message) (Utilities|Array|Get(acopy) _outactors (Math|Random|RandomIntegerinRange 0 (Utilities|Array|LastIndex _outactors)))))

(event EventReSpawnEndcaps
  ;[1 1 1] After all special rooms are spawned as well, time to spawn single-entrance dead end rooms on whatever probes we have left
  (Utilities|UpdateLoadingText "Mapping dead ends")
  ;;[1 0 0] ¯\_(ツ)_/¯
  (Utilities|FlowControl|Delay 0.1)
  (bind _outactors (Actor|GetAllActorsOfClass "/Game/Utility/BP_RoomSpawnProbe.BP_RoomSpawnProbe_C"))
  (for _array_element _outactors
    (Class|ISpawnsRooms|SpawnEndRoom(Message) _array_element))
  ;[1 1 1] Spawns doors between rooms
  (Utilities|UpdateLoadingText "Closing security doors")
  (bind _outactors_2 (Actor|GetAllActorsOfClass "/Game/Utility/DoorSpawner.DoorSpawner_C"))
  (for _array_element_2 _outactors_2
    (Class|ISpawnsDoors|SpawnDoor(Message) _array_element_2))
  ;[1 1 1] Sends a message to all Bps that have to do something on load end
  (Development|ExecuteConsoleCommand "RebuildNavigation")
  (bind _outactors_3 (Actor|GetAllActorswithInterface "/Game/Utility/I_LoadingEnds.I_LoadingEnds_C"))
  (for _array_element_3 _outactors_3
    (Class|ILoadingEnds|LoadingEnds(Message) _array_element_3)))

(event EventLoadingEnds
  ;[1 1 1] Cleanup
  ;;[1 0 0] ¯\_(ツ)_/¯
  (Utilities|FlowControl|Delay 1.0)
  ;;[1 1 1] Goes through all the probes again and tries to spawn dead end rooms again, because the 1st try sometimes fails ¯\_(ツ)_/¯
  (bind _outactors (Actor|GetAllActorsOfClass "/Game/Utility/BP_RoomSpawnProbe.BP_RoomSpawnProbe_C"))
  (for _array_element _outactors
    (Class|ISpawnsRooms|SpawnEndRoom(Message) _array_element)
    (Development|PrintString "2nd try"))
  ;;[1 1 1] Destroys all probes and kills itself
  (bind _outactors_2 (Actor|GetAllActorsOfClass "/Game/Utility/BP_RoomSpawnProbe.BP_RoomSpawnProbe_C"))
  (for _array_element_2 _outactors_2
    (Actor|DestroyActor _array_element_2)
    (Development|PrintString "Cleanup"))
  (Actor|DestroyActor))

(fn ConstructionScript)