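; Floor tile Blueprint that randomly knocks some tiles out of alignment to break up floor uniformity.
; The construction script rolls a random chance: most tiles stay in place with physics simulation switched off.
; The remaining minority get a random local offset and yaw rotation, keeping their default physics setting.
; The randomness is unseeded, and the event graph holds no active logic.
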(event EventBeginPlay)

(event Collision|EventActorBeginOverlap
  (params (OtherActor :type Actor%20Object%20Reference)))

(event EventTick
  (params (DeltaSeconds :type Float%20%28single-precision%29)))

(fn ConstructionScript
  (if (< (Math|Random|RandomIntegerinRange 0 100) 85)
    (Physics|SetSimulatePhysics (Variables|Default|GetTile) false)
    (else
      (Transformation|AddLocalOffset (Variables|Default|GetTile) (Math|Vector|MakeVector (Math|Random|RandomFloatinRange 15.0 6e+01) (Math|Random|RandomFloatinRange 15.0 6e+01) (Math|Random|RandomFloatinRange 5.0 1e+01)) false false)
      (Transformation|AddRelativeRotation (Variables|Default|GetTile) (Math|Rotator|MakeRotator 0.0 0.0 (Math|Random|RandomFloatinRange 0.0 3.6e+02)) false false))))