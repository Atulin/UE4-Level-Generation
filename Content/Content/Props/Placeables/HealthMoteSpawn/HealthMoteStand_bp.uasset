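; HealthMoteStand_bp is a placeable stand that spawns a pickup or prop on interaction: health mote, energy shield, money, bomb or keycard, chosen by WhatToSpawn.
; BeginPlay caches the spawn transform from its Sphere and color-codes the point light by type.
; The outer bounds enable spawning and show a tooltip that yaws toward the player each tick.
; The inner bounds hide the tooltip without disabling spawning.
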(event OnComponentBeginOverlap(InteractionBounds)
  (params (OverlappedComponent :type Primitive%20Component%20Object%20Reference) (OtherActor :type Actor%20Object%20Reference) (OtherComp :type Primitive%20Component%20Object%20Reference) (OtherBodyIndex :type Integer) (bFromSweep :type Boolean) (SweepResult :type Hit%20Result%20Structure%20%28by%20ref%29))
  ;[1 1 1] Hide & display tooltip
  (Variables|Default|SetCanSpawnMote true)
  (Rendering|SetVisibility (Variables|Default|GetWidget) true false))

(event OnComponentBeginOverlap(InnerInteractionBounds)
  (params (OverlappedComponent :type Primitive%20Component%20Object%20Reference) (OtherActor :type Actor%20Object%20Reference) (OtherComp :type Primitive%20Component%20Object%20Reference) (OtherBodyIndex :type Integer) (bFromSweep :type Boolean) (SweepResult :type Hit%20Result%20Structure%20%28by%20ref%29))
  ;[1 1 1] Hide & display tooltip
  (Rendering|SetVisibility (Variables|Default|GetWidget) false false))

(event OnComponentEndOverlap(InteractionBounds)
  (params (OverlappedComponent :type Primitive%20Component%20Object%20Reference) (OtherActor :type Actor%20Object%20Reference) (OtherComp :type Primitive%20Component%20Object%20Reference) (OtherBodyIndex :type Integer))
  ;[1 1 1] Hide & display tooltip
  (Variables|Default|SetCanSpawnMote false)
  (Rendering|SetVisibility (Variables|Default|GetWidget) false false))

(event OnComponentEndOverlap(InnerInteractionBounds)
  (params (OverlappedComponent :type Primitive%20Component%20Object%20Reference) (OtherActor :type Actor%20Object%20Reference) (OtherComp :type Primitive%20Component%20Object%20Reference) (OtherBodyIndex :type Integer))
  ;[1 1 1] Hide & display tooltip
  (Rendering|SetVisibility (Variables|Default|GetWidget) true false))

(event EventBeginPlay
  (bind _sphere (Variables|Default|GetSphere))
  (bind _returnvalue (Transformation|GetWorldTransform _sphere))
  (bind (_location _rotation) (Math|Transform|BreakTransform _returnvalue))
  (Rendering|SetVisibility (Variables|Default|GetWidget) false false)
  (Variables|Default|SetSpawnLocation (Math|Transform|MakeTransform _location _rotation))
  (switch string (Variables|Default|GetWhatToSpawn)
    (:health
      (Rendering|Components|Light|SetLightColor (Variables|Default|GetPointLight) "(R=1.000000,G=0.000000,B=0.000000,A=1.000000)" true))
    (:shield
      (Rendering|Components|Light|SetLightColor (Variables|Default|GetPointLight) "(R=1.000000,G=0.941987,B=0.290000,A=1.000000)" true))
    (:money
      (Rendering|Components|Light|SetLightColor (Variables|Default|GetPointLight) "(R=0.003254,G=1.000000,B=0.000000,A=1.000000)" true))
    (:bomb
      (Rendering|Components|Light|SetLightColor (Variables|Default|GetPointLight) "(R=1.000000,G=0.250082,B=0.000000,A=1.000000)" true))
    (:key
      (Rendering|Components|Light|SetLightColor (Variables|Default|GetPointLight) "(R=1.000000,G=1.000000,B=1.000000,A=1.000000)" true))))

(event EventTick
  (params (DeltaSeconds :type Float%20%28single-precision%29))
  (bind _widget (Variables|Default|GetWidget))
  ;[1 1 1] Rotate tooltip
  (Transformation|SetRelativeRotation _widget (Math|Rotator|MakeRotator 0.0 0.0 (.Yaw (Math|Rotator|BreakRotator (Math|Rotator|FindLookatRotation (Transformation|GetWorldLocation _widget) (Transformation|GetActorLocation (Game|Player|GetPlayerPawn 0)))))) false false))

(event EventInteract
  (params (PlayerRef :type First%20Person%20Character%20Object%20Reference))
  ;[1 1 1] Spawn Item
  (if (Variables|Default|GetCanSpawnMote)
    (switch string (Variables|Default|GetWhatToSpawn)
      (:health
        (Game|SpawnActorfromClass "/Game/Content/Props/Pickups/Healthpacks/HealthMote_bp.HealthMote_bp_C" (Variables|Default|GetSpawnLocation) "Undefined" 0 0 1e+01 0))
      (:shield
        (Game|SpawnActorfromClass "/Game/Content/Props/Pickups/Shield/BP_EnergyShield.BP_EnergyShield_C" (Variables|Default|GetSpawnLocation) "Undefined" 0 0))
      (:money
        (Game|SpawnActorfromClass "/Game/Content/Props/Pickups/Money/Money_bp.Money_bp_C" (Variables|Default|GetSpawnLocation) "Undefined" 0 10 100 0))
      (:bomb
        (Game|SpawnActorfromClass "/Game/Content/Props/Pickups/Bombs/BP_BombProp.BP_BombProp_C" (Variables|Default|GetSpawnLocation) "Undefined" 0 0))
      (:key
        (Game|SpawnActorfromClass "/Game/Content/Props/Pickups/Keycard/BP_Keycard.BP_Keycard_C" (Variables|Default|GetSpawnLocation) "Undefined" 0 0)))))

(fn ConstructionScript)