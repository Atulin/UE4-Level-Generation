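; BP_Door is a placeable door prop that opens on interaction or through open-all and close-all events.
; Interact and OpenAllDoor share one path that plays the door animation once and disables the Box collision.
; CloseAllDoor plays a separate backwards animation and restores query and physics collision.
; Both paths end in a game instance cast with nothing after it, and Interact only opens, never toggles.
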(event EventInteract
  (params (PlayerRef :type First%20Person%20Character%20Object%20Reference))
  (Components|Animation|PlayAnimation (Variables|Default|GetDoor1) "/Game/Content/Props/Placeables/Door/ANIM_Door.ANIM_Door" false)
  (Collision|SetCollisionEnabled (Variables|Default|GetBox) "NoCollision")
  (Utilities|Casting|CastToMyGameInstance (Game|GetGameInstance)))

(event EventOpenAllDoor
  (Components|Animation|PlayAnimation (Variables|Default|GetDoor1) "/Game/Content/Props/Placeables/Door/ANIM_Door.ANIM_Door" false)
  (Collision|SetCollisionEnabled (Variables|Default|GetBox) "NoCollision")
  (Utilities|Casting|CastToMyGameInstance (Game|GetGameInstance)))

(event EventCloseAllDoor
  (Components|Animation|PlayAnimation (Variables|Default|GetDoor1) "/Game/Content/Props/Placeables/Door/ANIM_DoorBackwards.ANIM_DoorBackwards" false)
  (Collision|SetCollisionEnabled (Variables|Default|GetBox) "QueryAndPhysics")
  (Utilities|Casting|CastToMyGameInstance (Game|GetGameInstance)))

(fn ConstructionScript)