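; BP_Bulkhead is a placeable bulkhead that replaces itself with a door when its surrounding line traces allow it.
; Three seconds after BeginPlay, two arrow traces must both hit, otherwise it logs a failure, spawns a BP_Marker and stays.
; If both hit, a short Raycast trace checks the hit actor's display name for "room".
; A match only prints that name; otherwise it spawns BP_Door at its transform and destroys itself.
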(event EventBeginPlay
  (bind _arrow (Variables|Default|GetArrow))
  (bind _arrow1 (Variables|Default|GetArrow1))
  (bind _defaultsceneroot (Variables|Default|GetDefaultSceneRoot))
  (bind _raycast (Variables|Default|GetRaycast))
  (bind _returnvalue (Transformation|GetWorldLocation _arrow))
  (bind _returnvalue_2 (Transformation|GetWorldLocation _raycast))
  (bind _returnvalue_3 (Transformation|GetWorldLocation _arrow1))
  (Utilities|FlowControl|Delay 3.0)
  (bind _returnvalue_4 (Collision|LineTraceByChannel _returnvalue (+ _returnvalue (* (Math|Vector|GetForwardVector _arrow) 250)) "TraceTypeQuery1" false 0 "None"))
  (Variables|Default|SetHit1 _returnvalue_4)
  (bind _returnvalue_5 (Collision|LineTraceByChannel _returnvalue_3 (+ _returnvalue_3 (* (Math|Vector|GetForwardVector _arrow1) 500)) "TraceTypeQuery1" false 0 "None"))
  (Variables|Default|SetHit2 _returnvalue_5)
  (if (and (Variables|Default|GetHit1) (Variables|Default|GetHit2))
    (bind _outhit (Collision|LineTraceByChannel _returnvalue_2 (+ _returnvalue_2 (* (Math|Vector|GetForwardVector _raycast) 50)) "TraceTypeQuery1" false 0 "ForDuration" true "(R=1.000000,G=0.000000,B=0.000000,A=1.000000)" "(R=0.000000,G=1.000000,B=0.000000,A=1.000000)" 1e+01))
    (if (Utilities|String|Contains (Utilities|GetDisplayName (.hitactor _outhit)) "room")
      (Development|PrintString (Utilities|GetDisplayName (.hitactor _outhit)) true true "(R=1.000000,G=0.000000,B=0.510845,A=1.000000)" 5.0)
      (else
        (Game|SpawnActorfromClass "/Game/Content/Props/Placeables/Door/BP_Door.BP_Door_C" (Transformation|GetWorldTransform (Variables|Default|GetDefaultSceneRoot)) "Undefined" 0 0)
        (Utilities|FlowControl|Delay 0.1)
        (Actor|DestroyActor)))
    (else
      (Development|PrintString "BULKHEAD NOT REPLACED" true true "(R=1.000000,G=0.033493,B=0.000000,A=1.000000)" 3e+01)
      (Game|SpawnActorfromClass "/Game/Utility/Marker/BP_Marker.BP_Marker_C" (Math|Transform|MakeTransform (* (Transformation|GetWorldLocation _defaultsceneroot) (* (Math|Vector|GetForwardVector _defaultsceneroot) 2)) (Transformation|GetWorldRotation _defaultsceneroot) "1,1,1") "AlwaysSpawn" 0 0))))

(fn ConstructionScript)