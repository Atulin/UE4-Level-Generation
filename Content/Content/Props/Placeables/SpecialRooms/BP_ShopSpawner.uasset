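; A placeholder actor that turns into one special room (shop, treasure or boss) at its location.
; On BeginPlay, if the Game Instance allows special rooms, it waits briefly, then spawns the first still-available type in shop, treasure, boss order.
; It clears that type's Game Instance flag so other spawners skip it, then destroys itself, as it does when nothing can spawn.
; A debug function prints the three flags before the delay.
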(event EventBeginPlay
  (bind _asmy_game_instance (Utilities|Casting|CastToMyGameInstance (Game|GetGameInstance)))
  (bind _output_get (Variables|Default|SetGameInstanceRef _asmy_game_instance))
  (if (Variables|/Game/Utility/MyGameInstance.MyGameInstance_C|GetCanSpecialRoomSpawn _output_get)
    (|Debug)
    (Utilities|FlowControl|Delay 0.2)
    (if (Variables|/Game/Utility/MyGameInstance.MyGameInstance_C|GetCanShopSpawn (Variables|Default|GetGameInstanceRef))
      (Variables|/Game/Utility/MyGameInstance.MyGameInstance_C|SetCanShopSpawn (Variables|Default|GetGameInstanceRef) false)
      (Game|SpawnActorfromClass "/Game/Content/Props/Placeables/SpecialRooms/BP_Shop.BP_Shop_C" (Transformation|GetWorldTransform (Variables|Default|GetDefaultSceneRoot)) "Undefined" 0 0)
      (Actor|DestroyActor :!label _label)
      (elif (Variables|/Game/Utility/MyGameInstance.MyGameInstance_C|GetCanTreasureSpawn (Variables|Default|GetGameInstanceRef))
        (Variables|/Game/Utility/MyGameInstance.MyGameInstance_C|SetCanTreasureSpawn (Variables|Default|GetGameInstanceRef) false)
        (Game|SpawnActorfromClass "/Game/Content/Props/Placeables/SpecialRooms/BP_Treasure.BP_Treasure_C" (Transformation|GetWorldTransform (Variables|Default|GetDefaultSceneRoot)) "Undefined" 0 0)
        (goto _label)
        (elif (Variables|/Game/Utility/MyGameInstance.MyGameInstance_C|GetCanBossSpawn (Variables|Default|GetGameInstanceRef))
          (Variables|/Game/Utility/MyGameInstance.MyGameInstance_C|SetCanBossSpawn (Variables|Default|GetGameInstanceRef) false)
          (Game|SpawnActorfromClass "/Game/Content/Props/Placeables/SpecialRooms/BP_Boss.BP_Boss_C" (Transformation|GetWorldTransform (Variables|Default|GetDefaultSceneRoot)) "Undefined" 0 0)
          (goto _label)
          (else
            (Actor|DestroyActor)))))
    (else
      (Actor|DestroyActor))))

(fn ConstructionScript)