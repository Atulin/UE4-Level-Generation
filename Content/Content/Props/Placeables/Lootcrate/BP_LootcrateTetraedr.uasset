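; Interactable loot crate that randomly becomes a rusty, ceramic or hex tier at BeginPlay, setting its material and beacon colour.
; A yaw-billboarded widget shows within the outer interaction bounds and hides inside the inner one.
; Interact works once, spawning a bomb, money, health, key or shield from tier-weighted odds, or a forced type, then plays an animation and removes the beacon.
; Tier also scales money and health amounts.
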(event OnComponentBeginOverlap(InteractionBounds)
  (params (OverlappedComponent :type Primitive%20Component%20Object%20Reference) (OtherActor :type Actor%20Object%20Reference) (OtherComp :type Primitive%20Component%20Object%20Reference) (OtherBodyIndex :type Integer) (bFromSweep :type Boolean) (SweepResult :type Hit%20Result%20Structure%20%28by%20ref%29))
  (if (Variables|Default|GetbCanInteract)
    (Rendering|SetVisibility (Variables|Default|GetWidget) true false)))

(event OnComponentBeginOverlap(InnerInteractionBounds)
  (params (OverlappedComponent :type Primitive%20Component%20Object%20Reference) (OtherActor :type Actor%20Object%20Reference) (OtherComp :type Primitive%20Component%20Object%20Reference) (OtherBodyIndex :type Integer) (bFromSweep :type Boolean) (SweepResult :type Hit%20Result%20Structure%20%28by%20ref%29))
  (Rendering|SetVisibility (Variables|Default|GetWidget) false false))

(event OnComponentEndOverlap(InteractionBounds)
  (params (OverlappedComponent :type Primitive%20Component%20Object%20Reference) (OtherActor :type Actor%20Object%20Reference) (OtherComp :type Primitive%20Component%20Object%20Reference) (OtherBodyIndex :type Integer))
  (Rendering|SetVisibility (Variables|Default|GetWidget) false false))

(event OnComponentEndOverlap(InnerInteractionBounds)
  (params (OverlappedComponent :type Primitive%20Component%20Object%20Reference) (OtherActor :type Actor%20Object%20Reference) (OtherComp :type Primitive%20Component%20Object%20Reference) (OtherBodyIndex :type Integer))
  (if (Variables|Default|GetbCanInteract)
    (Rendering|SetVisibility (Variables|Default|GetWidget) true false)))

(event EventInteract
  (params (PlayerRef :type First%20Person%20Character%20Object%20Reference))
  (bind _spawn (Variables|Default|GetSpawn))
  (bind _loottoforce (Variables|Default|GetLootToForce))
  (bind _returnvalue (Transformation|GetWorldTransform _spawn))
  (bind (_location _rotation) (Math|Transform|BreakTransform _returnvalue))
  (if (Variables|Default|GetbCanInteract)
    (Rendering|SetVisibility (Variables|Default|GetWidget) false false)
    (Variables|Default|SetbCanInteract false)
    (Variables|Default|SetSpawnLocation (Math|Transform|MakeTransform _location _rotation))
    (if (Variables|Config|GetbForceSpawnType)
      (if (Utilities|Enum|Equal(Enum) _loottoforce "bomb")
        (Utilities|SpawnBomb)
        (Utilities|PlayAnim :!label _label)
        (elif (Utilities|Enum|Equal(Enum) _loottoforce "money")
          (Utilities|SpawnMoney)
          (goto _label)
          (elif (Utilities|Enum|Equal(Enum) _loottoforce "health")
            (Utilities|SpawnHealth)
            (goto _label)
            (elif (Utilities|Enum|Equal(Enum) _loottoforce "key")
              (Utilities|SpawnKey)
              (goto _label)
              (elif (Utilities|Enum|Equal(Enum) _loottoforce "shield")
                (Utilities|SpawnShield)
                (goto _label))))))
      (elif (Utilities|Enum|Equal(Enum) (Variables|Default|GetCrateType) "rusty")
        (switch int (Math|Random|RandomIntegerinRange 0 2)
          (:0
            (Utilities|SpawnBomb))
          (:1
            (Utilities|SpawnMoney))
          (:2
            (Utilities|SpawnHealth)))
        (Utilities|PlayAnim)
        (elif (Utilities|Enum|Equal(Enum) (Variables|Default|GetCrateType) "ceramic")
          (switch int (Math|Random|RandomIntegerinRange 0 4)
            (:0
              (Utilities|SpawnBomb))
            (:1
              (Utilities|SpawnMoney :!label _label_2))
            (:2
              (goto _label_2))
            (:3
              (Utilities|SpawnHealth))
            (:4
              (Utilities|SpawnKey)))
          (Utilities|PlayAnim)
          (elif (Utilities|Enum|Equal(Enum) (Variables|Default|GetCrateType) "hex")
            (switch int (Math|Random|RandomIntegerinRange 0 6)
              (:0
                (Utilities|SpawnBomb))
              (:1
                (Utilities|SpawnMoney :!label _label_3))
              (:2
                (goto _label_3))
              (:3
                (Utilities|SpawnHealth))
              (:4
                (Utilities|SpawnKey :!label _label_4))
              (:5
                (goto _label_4))
              (:6
                (Utilities|SpawnShield)))
            (Utilities|PlayAnim)
            (else
              (Development|PrintString "NONEXISTENT CHEST" true true "(R=1.000000,G=0.000000,B=0.008842,A=1.000000)"))))))))

(event EventTick
  (params (DeltaSeconds :type Float%20%28single-precision%29))
  (bind _widget (Variables|Default|GetWidget))
  (Transformation|SetRelativeRotation _widget (Math|Rotator|MakeRotator 0.0 0.0 (.Yaw (Math|Rotator|BreakRotator (Math|Rotator|FindLookatRotation (Transformation|GetWorldLocation _widget) (Transformation|GetActorLocation (Game|Player|GetPlayerPawn 0)))))) false false))

(event EventBeginPlay
  (switch int (Math|Random|RandomIntegerinRange 0 8)
    (:0
      (Variables|Default|SetCrateType "rusty" :!label _label)
      (Rendering|Material|SetMaterial (Variables|Default|GetLootcrate_Tetraedr_uv) 0 "/Game/Content/Props/Placeables/Lootcrate/Rusty/LootcrateTetraedrRusty_mat.LootcrateTetraedrRusty_mat")
      (bind _returnvalue (Rendering|Material|CreateDynamicMaterialInstance (Variables|Default|GetCylinder) 0 "/Game/Content/Props/Placeables/Lootcrate/MAT_CrateBeacon.MAT_CrateBeacon" :!class /Script/Engine.PrimitiveComponent))
      (Rendering|Material|SetScalarParameterValue _returnvalue "Intensity" 3.0 :!class /Script/Engine.MaterialInstanceDynamic)
      (Rendering|Material|SetVectorParameterValue _returnvalue "Colour" "(R=1.000000,G=1.000000,B=1.000000,A=1.000000)" :!class /Script/Engine.MaterialInstanceDynamic))
    (:1
      (goto _label))
    (:2
      (goto _label))
    (:3
      (goto _label))
    (:4
      (Variables|Default|SetCrateType "ceramic" :!label _label_2)
      (Rendering|Material|SetMaterial (Variables|Default|GetLootcrate_Tetraedr_uv) 0 "/Game/Content/Props/Placeables/Lootcrate/Ceramic/LootcrateTetraedrCeramic_mat.LootcrateTetraedrCeramic_mat")
      (bind _returnvalue_2 (Rendering|Material|CreateDynamicMaterialInstance (Variables|Default|GetCylinder) 0 "/Game/Content/Props/Placeables/Lootcrate/MAT_CrateBeacon.MAT_CrateBeacon" :!class /Script/Engine.PrimitiveComponent))
      (Rendering|Material|SetScalarParameterValue _returnvalue_2 "Intensity" 3.0 :!class /Script/Engine.MaterialInstanceDynamic)
      (Rendering|Material|SetVectorParameterValue _returnvalue_2 "Colour" "(R=0.131763,G=1.000000,B=0.000000,A=1.000000)" :!class /Script/Engine.MaterialInstanceDynamic))
    (:5
      (goto _label_2))
    (:6
      (goto _label_2))
    (:7
      (Variables|Default|SetCrateType "hex" :!label _label_3)
      (Rendering|Material|SetMaterial (Variables|Default|GetLootcrate_Tetraedr_uv) 0 "/Game/Content/Props/Placeables/Lootcrate/Hex/LootcrateTetraedrHex_mat.LootcrateTetraedrHex_mat")
      (bind _returnvalue_3 (Rendering|Material|CreateDynamicMaterialInstance (Variables|Default|GetCylinder) 0 "/Game/Content/Props/Placeables/Lootcrate/MAT_CrateBeacon.MAT_CrateBeacon" :!class /Script/Engine.PrimitiveComponent))
      (Rendering|Material|SetScalarParameterValue _returnvalue_3 "Intensity" 3.0 :!class /Script/Engine.MaterialInstanceDynamic)
      (Rendering|Material|SetVectorParameterValue _returnvalue_3 "Colour" "(R=1.000000,G=0.680606,B=0.000000,A=1.000000)" :!class /Script/Engine.MaterialInstanceDynamic))
    (:8
      (goto _label_3)))
  (Rendering|SetVisibility (Variables|Default|GetWidget) false false))

(fn ConstructionScript)