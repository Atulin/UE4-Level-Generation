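; BP_Teleport is an interactable teleporter prop that sends the player to the level named in LoadLevel.
; Interact opens that level and resets the game instance's room locations, loading text and room count, using a reference cached on BeginPlay.
; Tick turns Sphere1 on yaw only to face the player.
; An older level-streaming path that flags loaded rooms for unload remains in the graph but is disconnected.
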(event EventBeginPlay
  (bind _asmy_game_instance (Utilities|Casting|CastToMyGameInstance (Game|GetGameInstance))
    (:then
      (Variables|Default|SetGameInstanceRef _asmy_game_instance))
    (:CastFailed
      (Development|PrintString "Cast to MyGameInstance failed" true true "(R=1.000000,G=0.000000,B=0.007957,A=1.000000)" 15.0))))

(event EventTick
  (params (DeltaSeconds :type Float%20%28single-precision%29))
  (bind _sphere1 (Variables|Default|GetSphere1))
  (Transformation|SetRelativeRotation _sphere1 (Math|Rotator|MakeRotator 0.0 0.0 (.Yaw (Math|Rotator|BreakRotator (Math|Rotator|FindLookatRotation (Transformation|GetWorldLocation _sphere1) (Transformation|GetActorLocation (Game|Player|GetPlayerPawn 0)))))) false false))

(event EventInteract
  (params (PlayerRef :type First%20Person%20Character%20Object%20Reference))
  (bind _gameinstanceref (Variables|Default|GetGameInstanceRef))
  (Game|OpenLevel(byName) (Variables|Default|GetLoadLevel))
  (Utilities|Array|Clear (Variables|/Game/Utility/MyGameInstance.MyGameInstance_C|GetRoomLocationsTakenInt _gameinstanceref))
  (Utilities|Array|Clear (Variables|/Game/Utility/MyGameInstance.MyGameInstance_C|GetLoadingText _gameinstanceref))
  (Variables|/Game/Utility/MyGameInstance.MyGameInstance_C|SetNumberOfRooms _gameinstanceref 0))

(fn ConstructionScript)