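; Target practice prop that topples when something overlaps its head or torso colliders, then resets.
; Each overlap prints debug text for the zone hit and feeds shared logic gated by IsToppled.
; For non-player actors, timelines roll the painted mesh relative to the Sphere's rotation, reversing after a delay and clearing the flag.
; The player pawn skips the rotation but still sets IsToppled, leaving it set.
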(event OnComponentBeginOverlap(HeadCollider)
  (params (OverlappedComponent :type Primitive%20Component%20Object%20Reference) (OtherActor :type Actor%20Object%20Reference) (OtherComp :type Primitive%20Component%20Object%20Reference) (OtherBodyIndex :type Integer) (bFromSweep :type Boolean) (SweepResult :type Hit%20Result%20Structure%20%28by%20ref%29))
  (bind _sphere (Variables|Default|GetSphere))
  (bind _sphere_2 (Variables|Default|GetSphere))
  (bind _returnvalue (Transformation|GetWorldRotation _sphere))
  (bind _returnvalue_2 (Transformation|GetWorldRotation _sphere_2))
  (bind (_roll _pitch _yaw) (Math|Rotator|BreakRotator _returnvalue))
  (bind (_roll_2 _pitch_2 _yaw_2) (Math|Rotator|BreakRotator _returnvalue_2))
  (Development|PrintString "You hit head!")
  (if (not (Variables|Default|GetIsToppled))
    (Variables|Default|SetIsToppled true)
    (if (not (== (stale OnComponentHit(TargetPractice_painted) OtherActor) (Game|Player|GetPlayerPawn 0)))
      (bind _smooth (Timeline|RotationTimeline PlayFromStart)
        (:Update
          (Transformation|SetWorldRotation (Variables|Default|GetTargetPractice_painted) (Math|Rotator|MakeRotator (- _roll _smooth) _pitch _yaw) false false)
          (Utilities|FlowControl|Delay 3.0)
          (bind _smooth_2 (Timeline|ResetTimeline PlayFromStart)
            (:Update
              (Transformation|SetWorldRotation (Variables|Default|GetTargetPractice_painted) (Math|Rotator|MakeRotator (+ _roll_2 _smooth_2) _pitch_2 _yaw_2) false false)
              (Variables|Default|SetIsToppled false))))))))

(event OnComponentBeginOverlap(TorsoCollider)
  (params (OverlappedComponent :type Primitive%20Component%20Object%20Reference) (OtherActor :type Actor%20Object%20Reference) (OtherComp :type Primitive%20Component%20Object%20Reference) (OtherBodyIndex :type Integer) (bFromSweep :type Boolean) (SweepResult :type Hit%20Result%20Structure%20%28by%20ref%29))
  (bind _sphere (Variables|Default|GetSphere))
  (bind _sphere_2 (Variables|Default|GetSphere))
  (bind _returnvalue (Transformation|GetWorldRotation _sphere))
  (bind _returnvalue_2 (Transformation|GetWorldRotation _sphere_2))
  (bind (_roll _pitch _yaw) (Math|Rotator|BreakRotator _returnvalue))
  (bind (_roll_2 _pitch_2 _yaw_2) (Math|Rotator|BreakRotator _returnvalue_2))
  (Development|PrintString "You hit torso!")
  (if (not (Variables|Default|GetIsToppled))
    (Variables|Default|SetIsToppled true)
    (if (not (== (stale OnComponentHit(TargetPractice_painted) OtherActor) (Game|Player|GetPlayerPawn 0)))
      (bind _smooth (Timeline|RotationTimeline PlayFromStart)
        (:Update
          (Transformation|SetWorldRotation (Variables|Default|GetTargetPractice_painted) (Math|Rotator|MakeRotator (- _roll _smooth) _pitch _yaw) false false)
          (Utilities|FlowControl|Delay 3.0)
          (bind _smooth_2 (Timeline|ResetTimeline PlayFromStart)
            (:Update
              (Transformation|SetWorldRotation (Variables|Default|GetTargetPractice_painted) (Math|Rotator|MakeRotator (+ _roll_2 _smooth_2) _pitch_2 _yaw_2) false false)
              (Variables|Default|SetIsToppled false))))))))

(event OnComponentBeginOverlap(TorsoCollider2)
  (params (OverlappedComponent :type Primitive%20Component%20Object%20Reference) (OtherActor :type Actor%20Object%20Reference) (OtherComp :type Primitive%20Component%20Object%20Reference) (OtherBodyIndex :type Integer) (bFromSweep :type Boolean) (SweepResult :type Hit%20Result%20Structure%20%28by%20ref%29))
  (bind _sphere (Variables|Default|GetSphere))
  (bind _sphere_2 (Variables|Default|GetSphere))
  (bind _returnvalue (Transformation|GetWorldRotation _sphere))
  (bind _returnvalue_2 (Transformation|GetWorldRotation _sphere_2))
  (bind (_roll _pitch _yaw) (Math|Rotator|BreakRotator _returnvalue))
  (bind (_roll_2 _pitch_2 _yaw_2) (Math|Rotator|BreakRotator _returnvalue_2))
  (Development|PrintString "You hit torso!")
  (if (not (Variables|Default|GetIsToppled))
    (Variables|Default|SetIsToppled true)
    (if (not (== (stale OnComponentHit(TargetPractice_painted) OtherActor) (Game|Player|GetPlayerPawn 0)))
      (bind _smooth (Timeline|RotationTimeline PlayFromStart)
        (:Update
          (Transformation|SetWorldRotation (Variables|Default|GetTargetPractice_painted) (Math|Rotator|MakeRotator (- _roll _smooth) _pitch _yaw) false false)
          (Utilities|FlowControl|Delay 3.0)
          (bind _smooth_2 (Timeline|ResetTimeline PlayFromStart)
            (:Update
              (Transformation|SetWorldRotation (Variables|Default|GetTargetPractice_painted) (Math|Rotator|MakeRotator (+ _roll_2 _smooth_2) _pitch_2 _yaw_2) false false)
              (Variables|Default|SetIsToppled false))))))))

(event OnComponentHit(TargetPractice_painted)
  (params (HitComponent :type Primitive%20Component%20Object%20Reference) (OtherActor :type Actor%20Object%20Reference) (OtherComp :type Primitive%20Component%20Object%20Reference) (NormalImpulse :type Vector :default "0, 0, 0") (Hit :type Hit%20Result%20Structure%20%28by%20ref%29)))

(fn ConstructionScript)