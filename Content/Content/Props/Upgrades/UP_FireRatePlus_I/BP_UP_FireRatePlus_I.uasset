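; Fire Rate Plus I upgrade pickup that cuts the player's FireRate value by 10% when collected.
; Interact and AttachAestheticUpgrade share one path that removes the sphere and rotating movement, resets the mesh transform and calls AttachUpgradeMessage on the player.
; The aesthetic entry sets a flag that skips the stat change.
; Both entries append the upgrade class to the game instance's AttachmentList.
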(event EventAttachAestheticUpgrade
  (params (PlayerRef :type First%20Person%20Character%20Object%20Reference))
  (Variables|Default|SetPlayerRef PlayerRef)
  (Variables|Default|SetbIsAestheticOnly true)
  (Components|DestroyComponent (Variables|Default|GetSphere))
  (Components|DestroyComponent (Variables|Default|GetRotatingMovement))
  (Transformation|ResetRelativeTransform (Variables|Default|GetFireRate01))
  (if (Variables|Default|GetbIsAestheticOnly)
    _
    (else
      (Variables|/Game/FirstPersonBP/FirstPersonCharacter.FirstPersonCharacter_C|SetFireRate (Variables|Default|GetPlayerRef) (- (Variables|/Game/FirstPersonBP/FirstPersonCharacter.FirstPersonCharacter_C|GetFireRate (Variables|Default|GetPlayerRef)) (* (Variables|/Game/FirstPersonBP/FirstPersonCharacter.FirstPersonCharacter_C|GetFireRate (Variables|Default|GetPlayerRef)) 0.1)))))
  (Class|IUpgrades|AttachUpgrade(Message) (Variables|Default|GetPlayerRef) self (Variables|Default|GetName) (Variables|Default|GetFlavour) (Variables|Default|GetbIsAestheticOnly))
  (bind _asmy_game_instance (Utilities|Casting|CastToMyGameInstance (Game|GetGameInstance)))
  (Utilities|Array|Add (Variables|/Game/Utility/MyGameInstance.MyGameInstance_C|GetAttachmentList _asmy_game_instance) (Variables|Default|GetUpgradeClass)))

(event EventInteract
  (params (PlayerRef :type First%20Person%20Character%20Object%20Reference))
  (Variables|Default|SetPlayerRef PlayerRef)
  (Components|DestroyComponent (Variables|Default|GetSphere))
  (Components|DestroyComponent (Variables|Default|GetRotatingMovement))
  (Transformation|ResetRelativeTransform (Variables|Default|GetFireRate01))
  (if (Variables|Default|GetbIsAestheticOnly)
    _
    (else
      (Variables|/Game/FirstPersonBP/FirstPersonCharacter.FirstPersonCharacter_C|SetFireRate (Variables|Default|GetPlayerRef) (- (Variables|/Game/FirstPersonBP/FirstPersonCharacter.FirstPersonCharacter_C|GetFireRate (Variables|Default|GetPlayerRef)) (* (Variables|/Game/FirstPersonBP/FirstPersonCharacter.FirstPersonCharacter_C|GetFireRate (Variables|Default|GetPlayerRef)) 0.1)))))
  (Class|IUpgrades|AttachUpgrade(Message) (Variables|Default|GetPlayerRef) self (Variables|Default|GetName) (Variables|Default|GetFlavour) (Variables|Default|GetbIsAestheticOnly))
  (bind _asmy_game_instance (Utilities|Casting|CastToMyGameInstance (Game|GetGameInstance)))
  (Utilities|Array|Add (Variables|/Game/Utility/MyGameInstance.MyGameInstance_C|GetAttachmentList _asmy_game_instance) (Variables|Default|GetUpgradeClass)))

(fn ConstructionScript)

(fn AttachUpgrade
  (params (UpgradeIn :type Actor%20Class%20Reference))
  (return))