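; Base Blueprint for upgrade pickups that attach to the player on interaction.
; Interact runs Initialize, which destroys the sphere and rotating movement components and resets the MagazineSize01 component's relative transform.
; Finalize then messages the player to attach the upgrade with its name, flavour and aesthetic-only flag, and records its class in MyGameInstance's AttachmentList.
; AttachUpgrade is an empty stub.
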(event EventInteract
  (params (PlayerRef :type First%20Person%20Character%20Object%20Reference))
  (CallFunction|Initialize PlayerRef)
  (CallFunction|Finalize PlayerRef))

(fn ConstructionScript)

(fn AttachUpgrade
  (params (UpgradeIn :type Actor%20Class%20Reference))
  (return))

(fn Initialize
  (params (PlayerRef :type First%20Person%20Character%20Object%20Reference))
  (Components|DestroyComponent (Variables|Default|GetSphere))
  (Components|DestroyComponent (Variables|Default|GetRotatingMovement))
  (Transformation|ResetRelativeTransform (Variables|Default|GetMagazineSize_01))
  (return (Variables|Default|GetbIsAestheticOnly)))

(fn Finalize
  (params (Target :type Object%20Object%20Reference))
  (Class|IUpgrades|AttachUpgrade(Message) Target self (Variables|Default|Getname) (Variables|Default|Getflavour) (Variables|Default|GetbIsAestheticOnly))
  (bind _asmy_game_instance (Utilities|Casting|CastToMyGameInstance (Game|GetGameInstance)))
  (Utilities|Array|Add (Variables|/Game/Utility/MyGameInstance.MyGameInstance_C|GetAttachmentList _asmy_game_instance) (Variables|Default|GetUpgradeClass)))