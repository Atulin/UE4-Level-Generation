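; Magazine-size upgrade pickup that adds five to the player's gun clip size, capped at 50, unless flagged as aesthetic-only.
; On Interact it removes its sphere and rotating movement, resets the magazine component's relative transform, and passes itself to the player's AttachUpgradeMessage.
; It also records its upgrade class in the game instance's AttachmentList.
; Its own AttachUpgrade function is an empty stub.
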(event EventInteract
  (params (PlayerRef :type First%20Person%20Character%20Object%20Reference))
  (Components|DestroyComponent (Variables|Default|GetSphere))
  (Components|DestroyComponent (Variables|Default|GetRotatingMovement))
  (Transformation|ResetRelativeTransform (Variables|Default|GetMagazineSize_01))
  (if (Variables|Default|GetbIsAestheticOnly)
    _
    (else
      (Variables|/Game/FirstPersonBP/FirstPersonCharacter.FirstPersonCharacter_C|SetGunClipSize PlayerRef (Math|Integer|Clamp(Integer) (+ (Variables|/Game/FirstPersonBP/FirstPersonCharacter.FirstPersonCharacter_C|GetGunClipSize PlayerRef) 5) 0 50))))
  (Class|IUpgrades|AttachUpgrade(Message) PlayerRef self (Variables|Default|Getname) (Variables|Default|Getflavour) (Variables|Default|GetbIsAestheticOnly))
  (bind _asmy_game_instance (Utilities|Casting|CastToMyGameInstance (Game|GetGameInstance)))
  (Utilities|Array|Add (Variables|/Game/Utility/MyGameInstance.MyGameInstance_C|GetAttachmentList _asmy_game_instance) (Variables|Default|GetUpgradeClass)))

(fn ConstructionScript)

(fn AttachUpgrade
  (params (UpgradeIn :type Actor%20Class%20Reference))
  (return))