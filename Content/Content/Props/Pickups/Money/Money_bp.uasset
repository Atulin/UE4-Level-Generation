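; Money pickup actor that grants the player a random amount of money when touched.
; On sphere overlap with a FirstPersonCharacter, it adds a random value between its minimum and maximum to PlayerMoney.
; It then looks up the HUD_Consumables widget by class to refresh the money display, and destroys itself.
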(event OnComponentBeginOverlap(Sphere)
  (params (OverlappedComponent :type Primitive%20Component%20Object%20Reference) (OtherActor :type Actor%20Object%20Reference) (OtherComp :type Primitive%20Component%20Object%20Reference) (OtherBodyIndex :type Integer) (bFromSweep :type Boolean) (SweepResult :type Hit%20Result%20Structure%20%28by%20ref%29))
  (bind _asfirst_person_character (Utilities|Casting|CastToFirstPersonCharacter OtherActor))
  (Variables|/Game/FirstPersonBP/FirstPersonCharacter.FirstPersonCharacter_C|SetPlayerMoney _asfirst_person_character (+ (Variables|/Game/FirstPersonBP/FirstPersonCharacter.FirstPersonCharacter_C|GetPlayerMoney _asfirst_person_character) (Math|Random|RandomIntegerinRange (Variables|Default|GetMinimumMoney) (Variables|Default|GetMaximumMoney))))
  (bind _foundwidgets (Widget|GetAllWidgetsOfClass "/Game/HUD/HUD_Consumables.HUD_Consumables_C" true))
  (Default|UpdateMoney (Utilities|Array|Get(acopy) _foundwidgets))
  (Actor|DestroyActor))

(fn ConstructionScript)