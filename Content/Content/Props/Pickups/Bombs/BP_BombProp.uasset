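; BP_BombProp is a bomb pickup that adds one bomb to the player's clamped count.
; A timeline started on BeginPlay drives the Bomb component's yaw, taking roll and pitch from the Sphere's world rotation.
; When a FirstPersonCharacter overlaps the Sphere, it increments Bombs, refreshes the first HUD_Consumables widget found by class lookup, and destroys itself.
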(event OnComponentBeginOverlap(Sphere)
  (params (OverlappedComponent :type Primitive%20Component%20Object%20Reference) (OtherActor :type Actor%20Object%20Reference) (OtherComp :type Primitive%20Component%20Object%20Reference) (OtherBodyIndex :type Integer) (bFromSweep :type Boolean) (SweepResult :type Hit%20Result%20Structure%20%28by%20ref%29))
  (bind _asfirst_person_character (Utilities|Casting|CastToFirstPersonCharacter OtherActor))
  (Variables|/Game/FirstPersonBP/FirstPersonCharacter.FirstPersonCharacter_C|SetBombs _asfirst_person_character (Math|Integer|Clamp(Integer) (+ (Variables|/Game/FirstPersonBP/FirstPersonCharacter.FirstPersonCharacter_C|GetBombs _asfirst_person_character) 1) 0 100))
  (bind _foundwidgets (Widget|GetAllWidgetsOfClass "/Game/HUD/HUD_Consumables.HUD_Consumables_C" true))
  (Default|UpdateBombs (Utilities|Array|Get(acopy) _foundwidgets))
  (Actor|DestroyActor))

(event EventBeginPlay
  (bind _sphere (Variables|Default|GetSphere))
  (bind _returnvalue (Transformation|GetWorldRotation _sphere))
  (bind _newtrack_0 (Timeline|Rotation PlayFromStart)
    (:Update
      (Transformation|SetRelativeRotation (Variables|Default|GetBomb) (Math|Rotator|MakeRotator (.roll _returnvalue) (.pitch _returnvalue) _newtrack_0) false false))))

(fn ConstructionScript)