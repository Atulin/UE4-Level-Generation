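; BP_EnergyShield is a pickup that restores a fixed amount of shield points to the first-person player character.
; On BeginPlay it caches the sphere's location and plays a timeline that lerps the actor vertically around that point for a bobbing effect.
; When a FirstPersonCharacter below max shield overlaps the sphere, it adds points clamped to the max, plays the healthpack sound and destroys itself.
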(event OnComponentBeginOverlap(Sphere)
  (params (OverlappedComponent :type Primitive%20Component%20Object%20Reference) (OtherActor :type Actor%20Object%20Reference) (OtherComp :type Primitive%20Component%20Object%20Reference) (OtherBodyIndex :type Integer) (bFromSweep :type Boolean) (SweepResult :type Hit%20Result%20Structure%20%28by%20ref%29))
  (bind _asfirst_person_character (Utilities|Casting|CastToFirstPersonCharacter OtherActor))
  (if (< (Variables|/Game/FirstPersonBP/FirstPersonCharacter.FirstPersonCharacter_C|GetPlayerShieldPoints _asfirst_person_character) (Variables|/Game/FirstPersonBP/FirstPersonCharacter.FirstPersonCharacter_C|GetPlayerShieldMax _asfirst_person_character))
    (Variables|/Game/FirstPersonBP/FirstPersonCharacter.FirstPersonCharacter_C|SetPlayerShieldPoints _asfirst_person_character (Math|Float|Clamp(Float) (+ (Variables|/Game/FirstPersonBP/FirstPersonCharacter.FirstPersonCharacter_C|GetPlayerShieldPoints _asfirst_person_character) 1e+01) 0.0 (Variables|/Game/FirstPersonBP/FirstPersonCharacter.FirstPersonCharacter_C|GetPlayerShieldMax _asfirst_person_character)))
    (Audio|PlaySoundatLocation "/Game/Content/Props/Pickups/Healthpacks/healthpack_sound.healthpack_sound" (Variables|Default|GetSpawnLocation) "0, 0, 0" 1.0 0.9)
    (Actor|DestroyActor)))

(event EventBeginPlay
  (bind _output_get (Variables|Default|SetSpawnLocation (Transformation|GetWorldLocation (Variables|Default|GetSphere))))
  (bind _positionz (Timeline|Timeline_0 Play)
    (:Update
      (Transformation|SetActorLocation (Math|Vector|Lerp(Vector) (Math|Vector|MakeVector (.X (Math|Vector|BreakVector _output_get)) (.Y (Math|Vector|BreakVector _output_get)) (+ (.Z (Math|Vector|BreakVector _output_get)) 5.0)) (Math|Vector|MakeVector (.X (Math|Vector|BreakVector _output_get)) (.Y (Math|Vector|BreakVector _output_get)) (- (.Z (Math|Vector|BreakVector _output_get)) 5.0)) _positionz) false false))))

(fn ConstructionScript)